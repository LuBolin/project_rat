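; BP_Mickey is a player-controlled Blueprint that connects Enhanced Input to movement, mouse pan and jump handlers.
; On BeginPlay it adds the IMC_Player mapping context to the owning player controller's local input subsystem.
; Each input action event forwards its action value to a matching CallFIA function, none of which is defined in this Blueprint.
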(event `self.ReceiveBeginPlay`
  ; Connect Input Mapping
  (bind _asplayer_controller (cast `PlayerController` (`self.GetController`)))
  (bind _returnvalue (pcsubsystem `EnhancedInputLocalPlayerSubsystem` _asplayer_controller))
  (`/Engine/EditorBlueprintResources/StandardMacros.IsValid` _returnvalue
    (:`Is Valid`
      (`EnhancedInputSubsystemInterface.AddMappingContext` _returnvalue "/Game/Player/Inputs/IMC_Player.IMC_Player" 0 (struct)))))

(event `EnhancedInput|/Game/Player/Inputs/IA_PlaneMovement`
  (params (ActionValue :type "Vector2D Structure") (ElapsedSeconds :type "Float (double-precision)") (TriggeredSeconds :type "Float (double-precision)") (InputAction :type "InputAction Object Reference" :default "/Game/Player/Inputs/IA_PlaneMovement.IA_PlaneMovement"))
  ; Input Event Binding
  (:`Triggered`
    (`self.FIA_PlaneMove` ActionValue)))

(event `EnhancedInput|/Game/Player/Inputs/IA_MousePan`
  (params (ActionValue :type "Vector2D Structure") (ElapsedSeconds :type "Float (double-precision)") (TriggeredSeconds :type "Float (double-precision)") (InputAction :type "InputAction Object Reference" :default "/Game/Player/Inputs/IA_MousePan.IA_MousePan"))
  ; Input Event Binding
  (:`Triggered`
    (`self.FIA_MousePan` ActionValue)))

(event `EnhancedInput|/Game/Player/Inputs/IA_Jump`
  (params (ActionValue :type Boolean) (ElapsedSeconds :type "Float (double-precision)") (TriggeredSeconds :type "Float (double-precision)") (InputAction :type "InputAction Object Reference" :default "/Game/Player/Inputs/IA_Jump.IA_Jump"))
  ; Input Event Binding
  (:`Triggered`
    (`self.FIA_Jump` ActionValue)))

(fn `UserConstructionScript`)